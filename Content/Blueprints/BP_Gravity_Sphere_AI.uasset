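; AI-driven gravity sphere that wanders, flees or charges the player depending on relative mass.
; A looping UpdateAI timer picks Wander, Panic or Attack from player distance and mass, and Tick runs that behavior.
; In Wander and Panic, Tick also scales the mesh by mass, makes heavier spheres static, and pulls movable ones toward the player with boostable inverse-square gravity.
; Overlaps add or remove the sphere as the player's attraction target.
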(event `self.ReceiveBeginPlay`
  (`self.SetActorEnableCollision` true)
  (bind _outactors (`GameplayStatics.GetAllActorsOfClass` "/Game/Blueprints/BP_ThirdPersonCharacter1.BP_ThirdPersonCharacter1_C"))
  (set `self.Player228` (`|GetArrayItem` _outactors))
  (`KismetSystemLibrary.K2_SetTimer` null "UpdateAI" 0.1 true true))

(event `self.ReceiveActorBeginOverlap`
  (params (OtherActor :type "Actor Object Reference"))
  (bind _asbp_third_person_character_1 (cast `/Game/Blueprints/BP_ThirdPersonCharacter1` OtherActor))
  (`/Game/Blueprints/BP_ThirdPersonCharacter1.Add Attraction Target` _asbp_third_person_character_1 self))

(event `self.ReceiveActorEndOverlap`
  (params (OtherActor :type "Actor Object Reference"))
  (bind _asbp_third_person_character_1 (cast `/Game/Blueprints/BP_ThirdPersonCharacter1` OtherActor))
  (`/Game/Blueprints/BP_ThirdPersonCharacter1.Remove Attraction Target` _asbp_third_person_character_1 self))

(event `self.ReceiveTick`
  (params (DeltaSeconds :type "Float (single-precision)"))
  (bind _player228 (`self.Player228`))
  (bind _returnvalue (- (`self.K2_GetActorLocation` _player228) (`self.K2_GetActorLocation`)))
  (switch `string` (`self.CurrentState`)
    (:`Panic`
      (`self.PanicBehavior` DeltaSeconds)
      (`SceneComponent.SetRelativeScale3D` (`self.StaticMeshComponent`) (`KismetMathLibrary.Conv_DoubleToVector` (`self.ObjectMass`)) :!label _label)
      (`self.UpdateFixPos`)
      (`/Engine/EditorBlueprintResources/StandardMacros.IsValid` _player228
        (:`Is Valid`
          (bind _asbp_third_person_character_1 (cast `/Game/Blueprints/BP_ThirdPersonCharacter1` (`self.Player228`)))
          (if (`/Game/Blueprints/BP_ThirdPersonCharacter1.IsGravityBoostActive` _asbp_third_person_character_1)
            (set `self.GravityPower` 50.0)
            (else
              (set `self.GravityPower` 10.0)))
          (if (== (`SceneComponent.Mobility` (`self.StaticMeshComponent`)) 2)
            (`PrimitiveComponent.AddForce` (`self.StaticMeshComponent`) (* (`KismetMathLibrary.Normal` _returnvalue) (* (/ (* (`self.GravityPower`) (`/Game/Blueprints/BP_ThirdPersonCharacter1.PlayerMass` _asbp_third_person_character_1)) (`KismetMathLibrary.Square` (`KismetMathLibrary.VSize` _returnvalue))) DeltaSeconds (`self.AttractionForce`) (`PrimitiveComponent.GetMass` (`self.StaticMeshComponent`)))) "None" false)))))
    (:`Wander`
      (`self.UpdateWanderBehavior` DeltaSeconds)
      (set `self.WanderTimer` (- (`self.WanderTimer`) DeltaSeconds))
      (goto _label))
    (:`Attack`
      (`self.AttackBehavior`))))

(fn `AttackBehavior`
  (`PrimitiveComponent.AddForce` (`self.StaticMeshComponent`) (* (`KismetMathLibrary.Normal` (- (`self.K2_GetActorLocation` (`self.Player228`)) (`self.K2_GetActorLocation`))) (`self.PanicSpeed`)) "None" false))

(fn `PanicBehavior`
  (params (DeltaTime :type "Float (double-precision)"))
  (`PrimitiveComponent.AddForce` (`self.StaticMeshComponent`) (* (`KismetMathLibrary.Normal` (- (`self.K2_GetActorLocation`) (`self.K2_GetActorLocation` (`self.Player228`)))) (`self.PanicSpeed`)) "None" false))

(fn `UpdateAI`
  (if (<= (`KismetMathLibrary.Vector_Distance` (`self.K2_GetActorLocation` (`self.Player228`)) (`self.K2_GetActorLocation`)) (`self.PanicRadius`))
    (bind _asbp_third_person_character_1 (cast `/Game/Blueprints/BP_ThirdPersonCharacter1` (`self.Player228`)))
    (if (>= (`/Game/Blueprints/BP_ThirdPersonCharacter1.PlayerMass` _asbp_third_person_character_1) (`self.ObjectMass`))
      (set `self.CurrentState` "Panic")
      (else
        (set `self.CurrentState` "Attack")))
    (else
      (set `self.CurrentState` "Wander"))))

(fn `UpdateFixPos`
  (bind _asbp_third_person_character_1 (cast `/Game/Blueprints/BP_ThirdPersonCharacter1` (`self.Player228`)))
  (if (> (`self.ObjectMass`) (`/Game/Blueprints/BP_ThirdPersonCharacter1.PlayerMass` _asbp_third_person_character_1))
    (`self.SetMobility` "Static")
    (else
      (`self.SetMobility` "Movable"))))

(fn `UpdateWanderBehavior`
  (params (DeltaTime :type "Float (double-precision)"))
  (if (<= (`self.WanderTimer`) 0.0)
    (set `self.WanderTimer` (`KismetMathLibrary.RandomFloatInRange` 0.5 3.0))
    (bind _output_get (set `self.WanderDirection` (`KismetMathLibrary.RandomUnitVector`))))
  (`self.K2_SetActorLocation` (+ (* _output_get (`self.WanderSpeed`) DeltaTime) (`self.K2_GetActorLocation`)))
  (`PrimitiveComponent.SetPhysicsLinearVelocity` (`self.StaticMeshComponent`) (0.0 0.0 0.0) false "None"))

(fn `UserConstructionScript`)