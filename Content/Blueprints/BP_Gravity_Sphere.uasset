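; Gravity body that registers as an attraction target on the player character while overlapping it and scales its mesh by ObjectMass.
; Each tick it turns static if heavier than the player, otherwise movable and pulled toward the player by an inverse-square, mass-based force.
; The player's gravity boost greatly strengthens that pull.
; LightAnim spawns green-material, collision-free copies with a given mesh and stores them in an array.
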(event `self.ReceiveBeginPlay`
  (`self.SetActorEnableCollision` true)
  (`KismetSystemLibrary.Delay` 0.2)
  (bind _asmaterial (cast `Material` (`PrimitiveComponent.GetMaterial` (`self.StaticMeshComponent`) 0)))
  (set `self.selfMaterial` _asmaterial))

(event `self.Sphere.OnComponentBeginOverlap`
  (params (OverlappedComponent :type "PrimitiveComponent Object Reference") (OtherActor :type "Actor Object Reference") (OtherComp :type "PrimitiveComponent Object Reference") (OtherBodyIndex :type Integer) (bFromSweep :type Boolean) (SweepResult :type "HitResult Structure (by ref)"))
  (bind _asbp_third_person_character_1 (cast `/Game/Blueprints/BP_ThirdPersonCharacter1` OtherActor :!label _label))
  (`/Game/Blueprints/BP_ThirdPersonCharacter1.Add Attraction Target` _asbp_third_person_character_1 self))

(event `self.ReceiveActorBeginOverlap`
  (params (OtherActor :type "Actor Object Reference"))
  (goto _label))

(event `self.ReceiveActorEndOverlap`
  (params (OtherActor :type "Actor Object Reference"))
  (bind _asbp_third_person_character_1 (cast `/Game/Blueprints/BP_ThirdPersonCharacter1` (stale `self.Sphere.OnComponentEndOverlap` OtherActor) :!label _label_2))
  (`/Game/Blueprints/BP_ThirdPersonCharacter1.Remove Attraction Target` _asbp_third_person_character_1 self))

(event `self.Sphere.OnComponentEndOverlap`
  (params (OverlappedComponent :type "PrimitiveComponent Object Reference") (OtherActor :type "Actor Object Reference") (OtherComp :type "PrimitiveComponent Object Reference") (OtherBodyIndex :type Integer))
  (goto _label_2))

(event `self.ReceiveTick`
  (params (DeltaSeconds :type "Float (single-precision)"))
  (bind _player228 (`self.Player228`))
  (bind _returnvalue (- (`self.K2_GetActorLocation` _player228) (`self.K2_GetActorLocation`)))
  (`SceneComponent.SetRelativeScale3D` (`self.StaticMeshComponent`) (`KismetMathLibrary.Conv_DoubleToVector` (`self.ObjectMass`)))
  (`self.UpdateFixPos`)
  (`/Engine/EditorBlueprintResources/StandardMacros.IsValid` _player228
    (:`Is Valid`
      (bind _asbp_third_person_character_1 (cast `/Game/Blueprints/BP_ThirdPersonCharacter1` (`self.Player228`)))
      (if (`/Game/Blueprints/BP_ThirdPersonCharacter1.IsGravityBoostActive` _asbp_third_person_character_1)
        (set `self.GravityPower` 50.0)
        (else
          (set `self.GravityPower` 3.0)))
      (if (== (`SceneComponent.Mobility` (`self.StaticMeshComponent`)) 2)
        (`PrimitiveComponent.AddForce` (`self.StaticMeshComponent`) (* (`KismetMathLibrary.Normal` _returnvalue) (* (/ (* (`self.ObjectMass`) (`/Game/Blueprints/BP_ThirdPersonCharacter1.PlayerMass` _asbp_third_person_character_1)) (`KismetMathLibrary.Square` (`KismetMathLibrary.VSize` _returnvalue))) DeltaSeconds (`self.AttractionForce`) (`PrimitiveComponent.GetMass` (`self.StaticMeshComponent`))) (`self.GravityPower`)) "None" false)))))

(fn `LightAnim`
  (params (SpawnPos :type "Vector Structure") (StaticMesh :type "StaticMesh Object Reference"))
  (bind _returnvalue (`|SpawnActorFromClass` "BP_Gravity_Sphere_C" (`KismetMathLibrary.Conv_VectorToTransform` SpawnPos) "Undefined" "MultiplyWithRoot" null null))
  (bind _staticmeshcomponent (`StaticMeshActor.StaticMeshComponent` _returnvalue))
  (`StaticMeshComponent.SetStaticMesh` _staticmeshcomponent StaticMesh)
  (`PrimitiveComponent.SetMaterial` _staticmeshcomponent 0 "/Game/MaterialsAndTextures/GreenLight.GreenLight")
  (set `PrimitiveComponent.bGenerateOverlapEvents` false _staticmeshcomponent)
  (`PrimitiveComponent.SetSimulatePhysics` _staticmeshcomponent false)
  (set `/Game/Blueprints/BP_Gravity_Sphere.Object Mass` 200.0 _returnvalue)
  (`PrimitiveComponent.SetCollisionEnabled` _staticmeshcomponent "NoCollision")
  (`KismetArrayLibrary.Array_Add` (`self.arrayOfCopies`) _returnvalue))

(fn `UpdateFixPos`
  (bind _asbp_third_person_character_1 (cast `/Game/Blueprints/BP_ThirdPersonCharacter1` (`self.Player228`)))
  (if (> (`self.ObjectMass`) (`/Game/Blueprints/BP_ThirdPersonCharacter1.PlayerMass` _asbp_third_person_character_1))
    (`self.SetMobility` "Static")
    (else
      (`self.SetMobility` "Movable"))))

(fn `UserConstructionScript`)