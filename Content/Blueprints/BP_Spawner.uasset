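; Spawner that populates the space level at BeginPlay with about a thousand randomized BP_Gravity_Sphere celestial bodies.
; It caches DT_SpaceObjects rows in a map by type, then CalculateChance makes a weighted roll for each body, though its BlackHole return is unreachable.
; GenerateObject assigns random mass and material from that data, scattering asteroids with random meshes around the player and other types across a far larger origin-centered volume.
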(event `self.ReceiveBeginPlay`
  (bind _outrownames (`DataTableFunctionLibrary.GetDataTableRowNames` "/Game/Data/DT_SpaceObjects.DT_SpaceObjects"))
  (for _array_element _outrownames
    (bind _returnvalue (`|GetDataTableRow` "/Game/Data/DT_SpaceObjects.DT_SpaceObjects" _array_element)
      (:`then`
        (if true
          (`BlueprintMapLibrary.Map_Add` (`self.CelestialDataMap`) (`KismetStringLibrary.Conv_StringToName` (`.Type_2_D9C4D05749183B4DDC9D8F92C786A533` (break `/Game/Data/Space_Objects_structure` _returnvalue))) _returnvalue)))))
  (`KismetSystemLibrary.Delay` 0.2)
  (for _ (range 1001)
    (bind _type (`self.CalculateChance`))
    (`self.GenerateObject` _type))
  (set `self.AllObjectsCreated` true))

(fn `CalculateChance`
  (returns (Type :type String))
  (bind _planetchance (`self.PlanetChance`))
  (bind _smallstarchance (`self.SmallStarChance`))
  (bind _mediumstarchance (`self.MediumStarChance`))
  (bind _bigstarchance (`self.BigStarChance`))
  (bind _asteroidchance (`self.AsteroidChance`))
  (bind _output_get (set `self.Total` (* (+ (`self.AsteroidChance`) (`self.PlanetChance`) (`self.SmallStarChance`) (`self.MediumStarChance`) (`self.BigStarChance`) (`self.GiantStarChance`) (`self.BlackHoleChance`)) (`KismetMathLibrary.RandomFloat`))))
  (if (< _output_get _asteroidchance)
    (return "Asteroid")
    (else
      (bind _output_get_2 (set `self.Total` (- (`self.Total`) _asteroidchance)))
      (if (< _output_get_2 _planetchance)
        (return "Planet")
        (else
          (bind _output_get_3 (set `self.Total` (- (`self.Total`) _planetchance)))
          (if (< _output_get_3 _smallstarchance)
            (return "SmallStar")
            (else
              (bind _output_get_4 (set `self.Total` (- (`self.Total`) _smallstarchance)))
              (if (< _output_get_4 _mediumstarchance)
                (return "MediumStar")
                (else
                  (bind _output_get_5 (set `self.Total` (- (`self.Total`) _mediumstarchance)))
                  (if (< _output_get_5 _bigstarchance)
                    (return "BigStar")
                    (else
                      (bind _output_get_6 (set `self.Total` (- (`self.Total`) _bigstarchance)))
                      (if (< _output_get_6 (`self.GiantStarChance`))
                        (return "GiantStar")))))))))))))

(fn `GenerateObject`
  (params (Type :type String))
  (bind (_value _returnvalue) (`BlueprintMapLibrary.Map_Find` (`self.CelestialDataMap`) (`KismetStringLibrary.Conv_StringToName` Type)))
  (bind (_type _minmass _maxmass _materials) (break `/Game/Data/Space_Objects_structure` _value))
  (if (`KismetStringLibrary.EqualEqual_StrStr` Type "Asteroid")
    (bind _asbp_third_person_character_1 (cast `/Game/Blueprints/BP_ThirdPersonCharacter1` (`self.Player`)))
    (bind _returnvalue_2 (`|SpawnActorFromClass` "/Game/Blueprints/BP_Gravity_Sphere.BP_Gravity_Sphere_C" (`KismetMathLibrary.Conv_VectorToTransform` (+ (`self.K2_GetActorLocation` _asbp_third_person_character_1) (`KismetMathLibrary.MakeVector` (`KismetMathLibrary.RandomFloatInRange` -200000.0 200000.0) (`KismetMathLibrary.RandomFloatInRange` -200000.0 200000.0) (`KismetMathLibrary.RandomFloatInRange` -200000.0 200000.0)))) "Undefined" "MultiplyWithRoot" null null))
    (`StaticMeshComponent.SetStaticMesh` (`StaticMeshActor.StaticMeshComponent` _returnvalue_2) (`KismetArrayLibrary.Array_Random` (`self.AsteroidMeshes`)))
    (set `/Game/Blueprints/BP_Gravity_Sphere.ObjectMass` (`KismetMathLibrary.RandomFloatInRange` _minmass _maxmass) _returnvalue_2)
    (`PrimitiveComponent.SetMaterial` (`StaticMeshActor.StaticMeshComponent` _returnvalue_2) 0 (`KismetArrayLibrary.Array_Random` _materials))
    (elif _returnvalue
      (bind _returnvalue_3 (`|SpawnActorFromClass` "/Game/Blueprints/BP_Gravity_Sphere.BP_Gravity_Sphere_C" (`KismetMathLibrary.Conv_VectorToTransform` (`KismetMathLibrary.MakeVector` (`KismetMathLibrary.RandomFloatInRange` -100000000.0 100000000.0) (`KismetMathLibrary.RandomFloatInRange` -100000000.0 100000000.0) (`KismetMathLibrary.RandomFloatInRange` -100000000.0 100000000.0))) "Undefined" "MultiplyWithRoot" null null))
      (set `/Game/Blueprints/BP_Gravity_Sphere.ObjectMass` (`KismetMathLibrary.RandomFloatInRange` _minmass _maxmass) _returnvalue_3)
      (`PrimitiveComponent.SetMaterial` (`StaticMeshActor.StaticMeshComponent` _returnvalue_3) 0 (`KismetArrayLibrary.Array_Random` _materials)))))

(fn `UserConstructionScript`)